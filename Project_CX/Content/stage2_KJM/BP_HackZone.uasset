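; BP_HackZone is a one-time trigger zone that runs an arrow-key hacking minigame while monsters keep spawning.
; The first box overlap starts a looping spawn timer at random spawn points, shows WBP_HackMinigame and enables input.
; Each round builds a random arrow sequence sized by RowLengths; correct keys turn green, while a mistake rerolls that round.
; Clearing all rounds stops spawning, destroys ExitDoor, removes the UI and disables input.
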(event OnComponentBeginOverlap(Box)
  (params (OverlappedComponent :type Primitive%20Component%20Object%20Reference) (OtherActor :type Actor%20Object%20Reference) (OtherComp :type Primitive%20Component%20Object%20Reference) (OtherBodyIndex :type Integer) (bFromSweep :type Boolean) (SweepResult :type Hit%20Result%20Structure%20%28by%20ref%29))
  (Utilities|FlowControl|DoOnce false
    (:Completed
      (Development|PrintString "해킹 시작")
      (bind _returnvalue (Utilities|Time|SetTimerbyEvent (delegate Custom|SpawnMonster) 3.0 true))
      (Variables|Default|SetSpawnTimer _returnvalue)
      (bind _returnvalue_2 (UserInterface|CreateWidget "/Game/stage2_KJM/WBP_HackMinigame.WBP_HackMinigame_C" (Game|GetPlayerController 0)))
      (bind _output_get (Variables|Default|SetHackUI _returnvalue_2))
      (UserInterface|Viewport|AddtoViewport _output_get 0)
      (Variables|Default|SetArrowTexts (Utilities|Array|MakeArray (Variables|/Game/stage2_KJM/WBP_HackMinigame.WBP_HackMinigame_C|GetArrow1 (Variables|Default|GetHackUI)) (Variables|/Game/stage2_KJM/WBP_HackMinigame.WBP_HackMinigame_C|GetArrow2 (Variables|Default|GetHackUI)) (Variables|/Game/stage2_KJM/WBP_HackMinigame.WBP_HackMinigame_C|GetArrow3 (Variables|Default|GetHackUI)) (Variables|/Game/stage2_KJM/WBP_HackMinigame.WBP_HackMinigame_C|GetArrow4 (Variables|Default|GetHackUI)) (Variables|/Game/stage2_KJM/WBP_HackMinigame.WBP_HackMinigame_C|GetArrow5 (Variables|Default|GetHackUI)) (Variables|/Game/stage2_KJM/WBP_HackMinigame.WBP_HackMinigame_C|GetArrow6 (Variables|Default|GetHackUI)) (Variables|/Game/stage2_KJM/WBP_HackMinigame.WBP_HackMinigame_C|GetArrow7 (Variables|Default|GetHackUI))))
      (CallFunction|NewRound)
      (Input|EnableInput (Game|GetPlayerController 0)))))

(event Custom|SpawnMonster
  (Game|SpawnActorfromClass (Variables|Default|GetMonsterClass) (Transformation|GetActorTransform (.OutItem (Utilities|Array|Random (Variables|Default|GetSpawnPoint)))) "AlwaysSpawn" "MultiplyWithRoot" 0 0))

(event Custom|NewRound
  (Utilities|Array|Clear (Variables|Default|GetSequence))
  (Variables|Default|SetInputIndex 0)
  (for _index (range 0 6)
    (if (< _index (Utilities|Array|Get(acopy) (Variables|Default|GetRowLengths) (Variables|Default|GetRound)))
      (Utilities|Array|Add (Variables|Default|GetSequence) (Math|Random|RandomInteger 4))
      (Variables|/Script/UMG.TextBlock|SetText (Utilities|Array|Get(acopy) (Variables|Default|GetArrowTexts) _index) (Utilities|Select :Index (Utilities|Array|Get(acopy) (Variables|Default|GetSequence) _index) :Option%200 "↑" :Option%201 "↓" :Option%202 "←" :Option%203 "→"))
      (Variables|/Script/UMG.TextBlock|SetColorAndOpacity (Utilities|Array|Get(acopy) (Variables|Default|GetArrowTexts) _index) (Utilities|Struct|MakeSlateColor "(R=1.000000,G=1.000000,B=1.000000,A=1.000000)"))
      (Variables|/Script/UMG.Widget|SetVisibility (Utilities|Array|Get(acopy) (Variables|Default|GetArrowTexts) _index) "Visible")
      (else
        (Variables|/Script/UMG.Widget|SetVisibility (Utilities|Array|Get(acopy) (Variables|Default|GetArrowTexts) _index) "Collapsed"))))
  (Variables|/Script/UMG.TextBlock|SetText (Variables|/Game/stage2_KJM/WBP_HackMinigame.WBP_HackMinigame_C|GetProgressText (Variables|Default|GetHackUI)) (Utilities|Text|FormatText "{0} / {1}" (Variables|Default|GetRound) (Utilities|Array|Length (Variables|Default|GetRowLengths)))))

(event Custom|CheckArrow
  (params (Dir :type Integer))
  (bind _inputindex (Variables|Default|GetInputIndex))
  (if (== (Utilities|Array|Get(acopy) (Variables|Default|GetSequence) _inputindex) Dir)
    (Variables|/Script/UMG.TextBlock|SetColorAndOpacity (Utilities|Array|Get(acopy) (Variables|Default|GetArrowTexts) _inputindex) (Utilities|Struct|MakeSlateColor "(R=0.040915,G=1.000000,B=0.144128,A=1.000000)"))
    (Math|Integer|IncrementInt _inputindex
      (:%20%20
        (if (== (Variables|Default|GetInputIndex) (Utilities|Array|Length (Variables|Default|GetSequence)))
          (bind _result (Math|Integer|IncrementInt (Variables|Default|GetRound))
            (:%20%20
              (if (== _result (Utilities|Array|Length (Variables|Default|GetRowLengths)))
                (CallFunction|HackComplete)
                (else
                  (CallFunction|NewRound))))))))
    (else
      (CallFunction|NewRound))))

(event Custom|HackComplete
  (Development|PrintString "해킹완료")
  (Utilities|Time|ClearandInvalidateTimerbyHandle (Variables|Default|GetSpawnTimer))
  (Actor|DestroyActor (Variables|Default|GetExitDoor))
  (Widget|RemovefromParent (Variables|Default|GetHackUI))
  (Input|DisableInput (Game|GetPlayerController 0)))

(event EventBeginPlay)

(event Collision|EventActorBeginOverlap
  (params (OtherActor :type Actor%20Object%20Reference)))

(event EventTick
  (params (DeltaSeconds :type Float%20%28single-precision%29)))

(event Input|KeyboardEvents|Up
  (params (Key :type Key%20Structure :default "None"))
  (:Pressed
    (CallFunction|CheckArrow)))

(event Input|KeyboardEvents|Down
  (params (Key :type Key%20Structure :default "None"))
  (:Pressed
    (CallFunction|CheckArrow 1)))

(event Input|KeyboardEvents|Left
  (params (Key :type Key%20Structure :default "None"))
  (:Pressed
    (CallFunction|CheckArrow 2)))

(event Input|KeyboardEvents|Right
  (params (Key :type Key%20Structure :default "None"))
  (:Pressed
    (CallFunction|CheckArrow 3)))

(fn ConstructionScript)